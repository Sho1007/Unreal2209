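; BP_TestZone is a named zone volume that sends its ZoneName to overlapping actors through EnterZoneMessage.
; On BeginPlay it sets itself as Owner of each valid zone in ChildZoneList, forming a parent-child hierarchy.
; Entering sends this zone's name, while leaving sends the owning parent zone's name, so nested zones fall back to the enclosing one.
; Leaving a zone without a BP_TestZone owner sends nothing.
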(event `self.ReceiveBeginPlay`
  (for _array_element (`self.ChildZoneList`)
    (`/Engine/EditorBlueprintResources/StandardMacros.IsValid` _array_element
      (:`Is Valid`
        (`self.SetOwner` _array_element self)))))

(event `self.ReceiveActorBeginOverlap`
  (params (OtherActor :type "Actor Object Reference"))
  (message `/Game/FormatText/Blueprints/IBP_Notice.EnterZone` OtherActor (`self.ZoneName`)))

(event `self.ReceiveActorEndOverlap`
  (params (OtherActor :type "Actor Object Reference"))
  (bind _asbp_test_zone (cast `/Game/FormatText/Blueprints/BP_TestZone` (`self.GetOwner`)))
  (message `/Game/FormatText/Blueprints/IBP_Notice.EnterZone` OtherActor (`/Game/FormatText/Blueprints/BP_TestZone.ZoneName` _asbp_test_zone)))

(fn `UserConstructionScript`)