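; BP_TestEnemy is a test enemy that can show a lock-on marker when targeted and react to damage.
; SetTargetWidget toggles the LockOnWidget, while SetText and TurnOff drive a VectorTestWidget that displays two numeric values.
; On damage it plays a hit-reaction animation directly on the mesh and prints the amount, skipping both while an animation is playing.
; Two getters expose IsDead, which nothing in these graphs sets.
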(event `/Game/TargetTut/Blueprints/IBP_Enemy.BP_SetTargetWidget`
  (params (bIsTargeted :type Boolean))
  (`SceneComponent.SetVisibility` (`self.LockOnWidget`) bIsTargeted false))

(event `TargetTut_EnemyInterface.SetTargetWidget`
  (params (bIsTargeted :type Boolean))
  (`SceneComponent.SetVisibility` (`self.LockOnWidget`) bIsTargeted false))

(event `self.ReceiveAnyDamage`
  (params (Damage :type "Float (single-precision)") (DamageType :type "DamageType Object Reference") (InstigatedBy :type "Controller Object Reference") (DamageCauser :type "Actor Object Reference"))
  (if (not (`SkeletalMeshComponent.IsPlaying` (`self.Mesh`)))
    (`SkeletalMeshComponent.PlayAnimation` (`self.Mesh`) "/Game/Resources/Animations/React/Standing_React_Large_From_Right_Anim.Standing_React_Large_From_Right_Anim" false)
    (`KismetSystemLibrary.PrintString` (`KismetStringLibrary.Conv_DoubleToString` Damage))))

(fn `BP_GetIsEnemyDead`
  (returns (bIsDead :type Boolean))
  (return (`self.bIsDead`)))

(fn `IsEnemyDead`
  (returns (ReturnValue :type Boolean))
  (return (`self.bIsDead`)))

(fn `SetText`
  (params (Input1 :type "Float (double-precision)") (Input2 :type "Float (double-precision)"))
  (bind _vectortestwidget (`self.VectorTestWidget`))
  (`SceneComponent.SetVisibility` _vectortestwidget true false)
  (bind _aswbp_vector_test (cast `/Game/InventoryTut/Widgets/WBP_VectorTest` (`WidgetComponent.GetUserWidgetObject` _vectortestwidget)))
  (`/Game/InventoryTut/Widgets/WBP_VectorTest.SetText` _aswbp_vector_test (`KismetTextLibrary.Conv_DoubleToText` (`local.Input1`) "HalfToEven"))
  (`/Game/InventoryTut/Widgets/WBP_VectorTest.SetText2` _aswbp_vector_test (`KismetTextLibrary.Conv_DoubleToText` (`local.Input2`) "HalfToEven")))

(fn `TurnOff`
  (`SceneComponent.SetVisibility` (`self.VectorTestWidget`) false false))

(fn `UserConstructionScript`)