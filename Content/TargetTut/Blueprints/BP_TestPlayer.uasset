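; BP_TestPlayer is a test player Blueprint for target lock-on, with clamped spring-arm camera zoom and a debug camera shake key.
; Input toggles lock-on or switches targets left and right, calling functions defined outside these graphs.
; EnterZone shows the zone name in a notice widget, with opacity driven by a timeline.
; TestFunc sphere-searches for test enemies, filters by a forward-angle threshold, and shows direction values on them.
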(event `InputAction|Zoom Camera In`
  (params (Key :type "Key Structure"))
  (bind _springarmcomponent (`self.SpringArmComponent`))
  ;[1 1 1] Camera Zoom In / Out
  (:`Pressed`
    (set `SpringArmComponent.TargetArmLength` (`KismetMathLibrary.FClamp` (- (`SpringArmComponent.TargetArmLength` _springarmcomponent) 20.0) 120.0 800.0) _springarmcomponent)))

(event `InputAction|Zoom Camera Out`
  (params (Key :type "Key Structure"))
  (bind _springarmcomponent (`self.SpringArmComponent`))
  ;[1 1 1] Camera Zoom In / Out
  (:`Pressed`
    (set `SpringArmComponent.TargetArmLength` (`KismetMathLibrary.FClamp` (+ (`SpringArmComponent.TargetArmLength` _springarmcomponent) 20.0) 120.0 800.0) _springarmcomponent)))

(event `self.ReceiveBeginPlay`
  ;[1 1 1] Notice Component
  (bind _returnvalue (`|CreateWidget` "/Game/FormatText/Widgets/WBP_Notice.WBP_Notice_C"))
  (bind _output_get (set `self.NoticeWidget` _returnvalue))
  (`UserWidget.AddToViewport` _output_get 0))

(event `InputAction|LockOn`
  (params (Key :type "Key Structure"))
  ;[1 1 1] LockOn Component Bind Input (추후 컴포넌트에 붙여야함)
  (:`Pressed`
    (if (`self.bIsLockOn`)
      (`self.LockOff`)
      (else
        (`self.LockOnTarget`)))))

(event `InputAction|SwitchTargetToLeft`
  (params (Key :type "Key Structure"))
  ;[1 1 1] LockOn Component Bind Input (추후 컴포넌트에 붙여야함)
  (:`Pressed`
    (if (`self.bIsLockOn`)
      (`self.LockOnLeftTarget`)
      (else
        (`self.LockOnTarget`)))))

(event `self.ReceiveTick`
  (params (DeltaSeconds :type "Float (single-precision)")))

(event `InputAction|SwitchTargetToRight`
  (params (Key :type "Key Structure"))
  ;[1 1 1] LockOn Component Bind Input (추후 컴포넌트에 붙여야함)
  (:`Pressed`
    (if (`self.bIsLockOn`)
      (`self.LockOnRightTarget`)
      (else
        (`self.LockOnTarget`)))))

(event `/Game/FormatText/Blueprints/IBP_Notice.EnterZone`
  (params (ZoneName :type Text))
  ;[1 1 1] Notice Component Widget Bind (추후 컴포넌트에 붙여야 함)
  (`/Game/FormatText/Widgets/WBP_Notice.SetText` (`self.NoticeWidget`) ZoneName)
  (bind (_direction `_새_트랙_0`) (`Timeline|타임라인_0` :!via `PlayFromStart`)
    (:`Update`
      (`/Game/FormatText/Widgets/WBP_Notice.SetTextOpacity` (`self.NoticeWidget`) `_새_트랙_0`))))

(event `Key|B`
  (params (Key :type "Key Structure"))
  (:`Pressed`
    (bind `_as플레이어_컨트롤러` (cast `PlayerController` (`self.GetController`)))
    (`PlayerCameraManager.StartCameraShake` :`self` (`PlayerController.PlayerCameraManager` `_as플레이어_컨트롤러`) :`ShakeClass` "/Game/TargetTut/Blueprints/BP_CameraShake.BP_CameraShake_C")))

(fn `TestFunc`
  (locals (NewLocalVar_0 :type "Array of Actor Object Reference"))
  (bind (_outactors _returnvalue) (`KismetSystemLibrary.SphereOverlapActors` (`self.K2_GetActorLocation`) 1000.0 (`|MakeArray` "ObjectTypeQuery3" :!type "EObjectTypeQuery Enum") "/Game/TargetTut/Blueprints/BP_TestEnemy.BP_TestEnemy_C"))
  (if _returnvalue
    (for _array_element _outactors
      (bind _asbp_test_enemy (cast `/Game/TargetTut/Blueprints/BP_TestEnemy` _array_element))
      (bind _returnvalue_2 (`self.K2_GetActorLocation` _array_element))
      (bind _result (`self.GetIsForward` _returnvalue_2))
      (if (> _result (`KismetMathLibrary.DegCos` (`self.TargetSearchDegrees`)))
        (bind _result_2 (`self.GetIsLeft` _returnvalue_2))
        (`/Game/TargetTut/Blueprints/BP_TestEnemy.SetText` _asbp_test_enemy _result_2 _result)
        (else
          (`/Game/TargetTut/Blueprints/BP_TestEnemy.TurnOff` _asbp_test_enemy))))))

(fn `UserConstructionScript`)