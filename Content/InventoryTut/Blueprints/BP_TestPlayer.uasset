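; BP_TestPlayer is a test player Blueprint prototyping camera-relative enemy lock-on, with mouse-look style axis input.
; Each Tick, it scans nearby BP_TestEnemy actors, using dot and cross products to show facing and side values on those within the view cone.
; LockOn toggles targeting: FindTargets picks the living enemy most aligned with the camera, searching only when DebugModeActive is set.
; LockOnCamera and LockOff are empty stubs.
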(event `self.ReceiveBeginPlay`)

(event `self.ReceiveTick`
  (params (DeltaSeconds :type "Float (single-precision)"))
  (`self.TestFunc`))

(event `InputAxis|LookUp`
  (params (AxisValue :type "Float (single-precision)"))
  (`self.AddControllerPitchInput` AxisValue))

(event `InputAxis|LookRight`
  (params (AxisValue :type "Float (single-precision)"))
  (`self.AddControllerYawInput` AxisValue))

(event `InputAction|LockOn`
  (params (Key :type "Key Structure"))
  (:`Pressed`
    (if (`self.bIsLockOn`)
      (`self.LockOff`)
      (else
        (`self.LockOnTarget`)))))

(fn `FindTargets`
  (locals (MaxValue :type "Float (double-precision)" :default 0.0) (SelectedActor :type "Actor Object Reference"))
  (bind (_outactors _returnvalue) (`KismetSystemLibrary.SphereOverlapActors` (`self.K2_GetActorLocation`) (`self.TargetSearchRadius`) (`|MakeArray` "ObjectTypeQuery3" :!type "EObjectTypeQuery Enum") "/Game/InventoryTut/Blueprints/BP_TestEnemy.BP_TestEnemy_C" (`|MakeArray` self :!type "Actor Object Reference")))
  ;[1 1 1] Draw Debug Sphere
  (if (`self.bDebugModeActive`)
    (`KismetSystemLibrary.DrawDebugSphere` (`self.K2_GetActorLocation`) (`self.TargetSearchRadius`) 12 (struct :`G` 1.0 :`B` 0.094754 :`A` 1.0) 5.0 5.0)
    ;[1 1 1] Set Potential Targets
    (if _returnvalue
      (for _array_element _outactors
        (bind _bisdead (message `/Game/InventoryTut/Blueprints/IBP_Enemy.GetIsEnemyDead` _array_element))
        (if (not _bisdead)
          (`KismetArrayLibrary.Array_AddUnique` (`self.PotentialTargets`) _array_element)))
      ;[1 1 1] Select Target
      (for _array_element_2 (`self.PotentialTargets`)
        (bind _result (`self.GetIsForward` (`self.K2_GetActorLocation` _array_element_2)))
        (if (> _result (`local.MaxValue`))
          (set `local.MaxValue` _result)
          (set `local.SelectedActor` _array_element_2)))
      (bind _selectedactor (`local.SelectedActor`)
        (:`then`
          (set `self.TargetLocked` _selectedactor)
          (return))
        (:`else`)))))

(fn `GetIsForward`
  (params (TargetLocation :type "Vector Structure"))
  (returns (Result :type "Float (double-precision)"))
  (bind _returnvalue (- TargetLocation (`SceneComponent.K2_GetComponentLocation` (`self.Camera`))))
  (return (/ (`KismetMathLibrary.Dot_VectorVector` _returnvalue (`SceneComponent.GetForwardVector` (`self.Camera`))) (`KismetMathLibrary.VSize` _returnvalue))))

(fn `GetIsLeft`
  (params (TargetLocation :type "Vector Structure"))
  (returns (Result :type "Float (double-precision)"))
  (return (`KismetMathLibrary.Dot_VectorVector` (`KismetMathLibrary.Cross_VectorVector` (- TargetLocation (`SceneComponent.K2_GetComponentLocation` (`self.Camera`))) (`SceneComponent.GetForwardVector` (`self.Camera`))) (`SceneComponent.GetUpVector` (`self.Camera`)))))

(fn `LockOff`)

(fn `LockOnCamera`)

(fn `LockOnTarget`
  ;[1 1 1] Double Check
  (if (not (`self.bIsLockOn`))
    (`self.FindTargets`)
    (`self.TargetLocked`
      (:`then`
        (`self.LockOnCamera`)
        (bind _output_get (set `self.bIsLockOn` true))
        (bind _output_get_2 (set `self.bIsCameraLocked` _output_get))
        (message `/Game/InventoryTut/Blueprints/IBP_Enemy.SetTargetWidget` (`self.TargetLocked`) _output_get_2))
      (:`else`
        (`self.LockOff` :!label _label)))
    (else
      (goto _label))))

(fn `TestFunc`
  (locals (NewLocalVar_0 :type "Array of Actor Object Reference"))
  (bind _newlocalvar_0 (`local.NewLocalVar_0`))
  (`KismetArrayLibrary.Array_Add` _newlocalvar_0 self)
  (bind (_outactors _returnvalue) (`KismetSystemLibrary.SphereOverlapActors` (`self.K2_GetActorLocation`) 1000.0 (`self.Object Types`) "/Game/InventoryTut/Blueprints/BP_TestEnemy.BP_TestEnemy_C" _newlocalvar_0))
  (if _returnvalue
    (for _array_element _outactors
      (bind _asbp_test_enemy (cast `/Game/InventoryTut/Blueprints/BP_TestEnemy` _array_element))
      (bind _returnvalue_2 (`self.K2_GetActorLocation` _array_element))
      (bind _result (`self.GetIsForward` _returnvalue_2))
      (if (> _result (`KismetMathLibrary.DegCos` (`self.TargetSearchDegree`)))
        (bind _result_2 (`self.GetIsLeft` _returnvalue_2))
        (`/Game/InventoryTut/Blueprints/BP_TestEnemy.SetText` _asbp_test_enemy _result_2 _result)
        (else
          (`/Game/InventoryTut/Blueprints/BP_TestEnemy.TurnOff` _asbp_test_enemy))))))

(fn `UserConstructionScript`)