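; BP_NPC is an AI-driven melee character that spawns a goblin axe on its hand socket and destroys it along with itself.
; On BeginPlay it seeds the Blackboard with patrol wait time and attack range.
; MeleeAttack plays a slash montage whose notify triggers a forward sphere trace to apply damage.
; Incoming damage goes to the status component, which also receives sprint state when walk speed is updated.
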(event `self.ReceiveBeginPlay`
  (bind _returnvalue (`AIBlueprintHelperLibrary.GetBlackboard` null))
  (`BlackboardComponent.SetValueAsFloat` _returnvalue "WaitTime" (`/Game/AI/NPC/BP_PatrolPath.WaitTime` (`self.PatrolPath`)))
  (`BlackboardComponent.SetValueAsFloat` _returnvalue "AttackRange" 150.0)
  (bind _returnvalue_2 (`|SpawnActorFromClass` "/Game/AI/NPC/BP_GoblinAxe.BP_GoblinAxe_C" (`SceneComponent.GetSocketTransform` (`self.Mesh`) "WeaponSocket" "RTS_World") "Undefined" "OverrideRootScale" null null))
  (bind _output_get (set `self.Weapon` _returnvalue_2))
  (`self.K2_AttachToComponent` _output_get (`self.Mesh`) "WeaponSocket" "SnapToTarget" "SnapToTarget" "SnapToTarget" true))

(event `self.ReceiveAnyDamage`
  (params (Damage :type "Float (single-precision)") (DamageType :type "DamageType Object Reference") (InstigatedBy :type "Controller Object Reference") (DamageCauser :type "Actor Object Reference"))
  (`CharacterStatusComponent.RecieveDamage` (`self.AC_TestCharacterStatus`) Damage))

(event `/Game/AI/NPC/IBP_Combat.MeleeAttack`
  (params (TargetLocation :type "Vector Structure"))
  (bind _returnvalue (`self.K2_GetActorLocation`))
  (`|PlayMontage` (`self.Mesh`) "/Game/TargetTut/Animations/Goblin_Male/AM_GoblinMale_Slash.AM_GoblinMale_Slash"
    (:`OnNotifyBegin`
      (bind (_outhit _returnvalue_2) (`KismetSystemLibrary.SphereTraceSingle` _returnvalue (+ _returnvalue (* (`self.GetActorForwardVector`) 180.0)) 50.0 "TraceTypeQuery2"))
      (if _returnvalue_2
        (`GameplayStatics.ApplyDamage` (`.HitActor` (`GameplayStatics.BreakHitResult` _outhit)) 50.0 null self)))))

(event `self.ReceiveDestroyed`
  (`self.K2_DestroyActor` (`self.Weapon`)))

(fn `Update Walk Speed`
  (params (Value :type "Float (double-precision)") (bIsSprint :type Boolean))
  (set `CharacterMovementComponent.MaxWalkSpeed` Value (`self.CharacterMovement`))
  (set `CharacterStatusComponent.bIsSprint` bIsSprint (`self.AC_TestCharacterStatus`)))

(fn `UserConstructionScript`)