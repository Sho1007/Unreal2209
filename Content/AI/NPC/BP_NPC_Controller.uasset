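; BP_NPC_Controller is an NPC AI controller that runs the BT_NPC behavior tree on BeginPlay.
; On each perception update, it looks for an AC_TestCharacterStatus component on the perceived actor.
; If one exists, its IsDead flag sets the bIsTargetDead blackboard key, and the inverse sets bCanSeePlayer.
; The stimulus is not checked, so losing perception of a living target still sets bCanSeePlayer true.
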(event `self.ReceiveBeginPlay`
  (`self.RunBehaviorTree` "/Game/AI/NPC/BT_NPC.BT_NPC"))

(event `self.AIPerception.OnTargetPerceptionUpdated`
  (params (Actor :type "Actor Object Reference") (Stimulus :type "AIStimulus Structure"))
  (bind _returnvalue (`self.GetComponentByClass` Actor "/Game/Damage_Healing/Blueprints/AC_TestCharacterStatus.AC_TestCharacterStatus_C"))
  (bind _bisdead (`CharacterStatusComponent.bIsDead` _returnvalue))
  (`/Engine/EditorBlueprintResources/StandardMacros.IsValid` _returnvalue
    (:`Is Valid`
      (`BlackboardComponent.SetValueAsBool` (`self.Blackboard`) "bCanSeePlayer" (not _bisdead))
      (`BlackboardComponent.SetValueAsBool` (`self.Blackboard`) "bIsTargetDead" _bisdead))))

(fn `UserConstructionScript`)